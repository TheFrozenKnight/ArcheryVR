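; BP_HE_Ballon_Dynamic is a VR archery hitting element that acts as a recurring balloon spawner.
; On BeginPlay it spawns a BP_Ballon at its Balloon component's world transform, then repeats on a looping timer.
; Each new balloon goes through RefreshMaterial, which casts it and applies a randomly picked material from the Color array to its static mesh.
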(event `self.ReceiveBeginPlay`
  (`self.CreateBalloon`)
  (`KismetSystemLibrary.K2_SetTimer` null "CreateBalloon" 10.0 true))

(fn `CreateBalloon`
  (bind _returnvalue (`|SpawnActorFromClass` "/Game/VR_Archery/Blueprint/HittingElement/BP_Ballon.BP_Ballon_C" (`SceneComponent.K2_GetComponentToWorld` (`self.Balloon`)) "Undefined" "OverrideRootScale" null null))
  (`self.RefreshMaterial` _returnvalue))

(fn `RefreshMaterial`
  (params (Ballon :type "StaticMeshActor Object Reference"))
  (bind _asbp_ballon (cast `/Game/VR_Archery/Blueprint/HittingElement/BP_Ballon` Ballon))
  (`PrimitiveComponent.SetMaterial` (`StaticMeshActor.StaticMeshComponent` _asbp_ballon) 0 (`|GetArrayItem` (`self. Color`) (`KismetMathLibrary.RandomInteger` 6))))

(fn `UserConstructionScript`)