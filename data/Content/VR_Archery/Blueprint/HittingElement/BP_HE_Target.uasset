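; VR archery target that awards 1 to 10 points according to which of its ten ring meshes an arrow hits.
; Each ring's overlap event calls Shoot, which matches "ArrowBox" in the component's name, casts to BP_Arrow and disables that box's collision.
; A successful hit adds the ring's value to TotalScore, updates the score TextRender and plays the AHitTarget sound.
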(event `self.SM_Ring_1.OnComponentBeginOverlap`
  (params (OverlappedComponent :type "PrimitiveComponent Object Reference") (OtherActor :type "Actor Object Reference") (OtherComp :type "PrimitiveComponent Object Reference") (OtherBodyIndex :type Integer) (bFromSweep :type Boolean) (SweepResult :type "HitResult Structure (by ref)"))
  (bind _returnvalue (+ (`self.TotalScore`) 1))
  (bind _isshoot (`self.Shoot` OtherActor OtherComp))
  (if _isshoot
    (set `self.TotalScore` _returnvalue)
    (`TextRenderComponent.K2_SetText` (`self.TextRender`) (`|FormatText` "Score: {score}" _returnvalue))
    (`AudioComponent.Play` (`self.A_HitTarget`) 0.0 :!label _label)))

(event `self.SM_Ring_2.OnComponentBeginOverlap`
  (params (OverlappedComponent :type "PrimitiveComponent Object Reference") (OtherActor :type "Actor Object Reference") (OtherComp :type "PrimitiveComponent Object Reference") (OtherBodyIndex :type Integer) (bFromSweep :type Boolean) (SweepResult :type "HitResult Structure (by ref)"))
  (bind _returnvalue (+ (`self.TotalScore`) 2))
  (bind _isshoot (`self.Shoot` OtherActor OtherComp))
  (if _isshoot
    (set `self.TotalScore` _returnvalue)
    (`TextRenderComponent.K2_SetText` (`self.TextRender`) (`|FormatText` "Score: {score}" _returnvalue))
    (goto _label)))

(event `self.SM_Ring_3.OnComponentBeginOverlap`
  (params (OverlappedComponent :type "PrimitiveComponent Object Reference") (OtherActor :type "Actor Object Reference") (OtherComp :type "PrimitiveComponent Object Reference") (OtherBodyIndex :type Integer) (bFromSweep :type Boolean) (SweepResult :type "HitResult Structure (by ref)"))
  (bind _returnvalue (+ (`self.TotalScore`) 3))
  (bind _isshoot (`self.Shoot` OtherActor OtherComp))
  (if _isshoot
    (set `self.TotalScore` _returnvalue)
    (`TextRenderComponent.K2_SetText` (`self.TextRender`) (`|FormatText` "Score: {score}" _returnvalue))
    (goto _label)))

(event `self.SM_Ring_4.OnComponentBeginOverlap`
  (params (OverlappedComponent :type "PrimitiveComponent Object Reference") (OtherActor :type "Actor Object Reference") (OtherComp :type "PrimitiveComponent Object Reference") (OtherBodyIndex :type Integer) (bFromSweep :type Boolean) (SweepResult :type "HitResult Structure (by ref)"))
  (bind _returnvalue (+ (`self.TotalScore`) 4))
  (bind _isshoot (`self.Shoot` OtherActor OtherComp))
  (if _isshoot
    (set `self.TotalScore` _returnvalue)
    (`TextRenderComponent.K2_SetText` (`self.TextRender`) (`|FormatText` "Score: {score}" _returnvalue))
    (goto _label)))

(event `self.SM_Ring_5.OnComponentBeginOverlap`
  (params (OverlappedComponent :type "PrimitiveComponent Object Reference") (OtherActor :type "Actor Object Reference") (OtherComp :type "PrimitiveComponent Object Reference") (OtherBodyIndex :type Integer) (bFromSweep :type Boolean) (SweepResult :type "HitResult Structure (by ref)"))
  (bind _returnvalue (+ (`self.TotalScore`) 5))
  (bind _isshoot (`self.Shoot` OtherActor OtherComp))
  (if _isshoot
    (set `self.TotalScore` _returnvalue)
    (`TextRenderComponent.K2_SetText` (`self.TextRender`) (`|FormatText` "Score: {score}" _returnvalue))
    (goto _label)))

(event `self.SM_Ring_6.OnComponentBeginOverlap`
  (params (OverlappedComponent :type "PrimitiveComponent Object Reference") (OtherActor :type "Actor Object Reference") (OtherComp :type "PrimitiveComponent Object Reference") (OtherBodyIndex :type Integer) (bFromSweep :type Boolean) (SweepResult :type "HitResult Structure (by ref)"))
  (bind _returnvalue (+ (`self.TotalScore`) 6))
  (bind _isshoot (`self.Shoot` OtherActor OtherComp))
  (if _isshoot
    (set `self.TotalScore` _returnvalue)
    (`TextRenderComponent.K2_SetText` (`self.TextRender`) (`|FormatText` "Score: {score}" _returnvalue))
    (goto _label)))

(event `self.SM_Ring_7.OnComponentBeginOverlap`
  (params (OverlappedComponent :type "PrimitiveComponent Object Reference") (OtherActor :type "Actor Object Reference") (OtherComp :type "PrimitiveComponent Object Reference") (OtherBodyIndex :type Integer) (bFromSweep :type Boolean) (SweepResult :type "HitResult Structure (by ref)"))
  (bind _returnvalue (+ (`self.TotalScore`) 7))
  (bind _isshoot (`self.Shoot` OtherActor OtherComp))
  (if _isshoot
    (set `self.TotalScore` _returnvalue)
    (`TextRenderComponent.K2_SetText` (`self.TextRender`) (`|FormatText` "Score: {score}" _returnvalue))
    (goto _label)))

(event `self.SM_Ring_8.OnComponentBeginOverlap`
  (params (OverlappedComponent :type "PrimitiveComponent Object Reference") (OtherActor :type "Actor Object Reference") (OtherComp :type "PrimitiveComponent Object Reference") (OtherBodyIndex :type Integer) (bFromSweep :type Boolean) (SweepResult :type "HitResult Structure (by ref)"))
  (bind _returnvalue (+ (`self.TotalScore`) 8))
  (bind _isshoot (`self.Shoot` OtherActor OtherComp))
  (if _isshoot
    (set `self.TotalScore` _returnvalue)
    (`TextRenderComponent.K2_SetText` (`self.TextRender`) (`|FormatText` "Score: {score}" _returnvalue))
    (goto _label)))

(event `self.SM_Ring_9.OnComponentBeginOverlap`
  (params (OverlappedComponent :type "PrimitiveComponent Object Reference") (OtherActor :type "Actor Object Reference") (OtherComp :type "PrimitiveComponent Object Reference") (OtherBodyIndex :type Integer) (bFromSweep :type Boolean) (SweepResult :type "HitResult Structure (by ref)"))
  (bind _returnvalue (+ (`self.TotalScore`) 9))
  (bind _isshoot (`self.Shoot` OtherActor OtherComp))
  (if _isshoot
    (set `self.TotalScore` _returnvalue)
    (`TextRenderComponent.K2_SetText` (`self.TextRender`) (`|FormatText` "Score: {score}" _returnvalue))
    (goto _label)))

(event `self.SM_Ring_10.OnComponentBeginOverlap`
  (params (OverlappedComponent :type "PrimitiveComponent Object Reference") (OtherActor :type "Actor Object Reference") (OtherComp :type "PrimitiveComponent Object Reference") (OtherBodyIndex :type Integer) (bFromSweep :type Boolean) (SweepResult :type "HitResult Structure (by ref)"))
  (bind _returnvalue (+ (`self.TotalScore`) 10))
  (bind _isshoot (`self.Shoot` OtherActor OtherComp))
  (if _isshoot
    (set `self.TotalScore` _returnvalue)
    (`TextRenderComponent.K2_SetText` (`self.TextRender`) (`|FormatText` "Score: {score}" _returnvalue))
    (goto _label)))

(fn `Shoot`
  (params (OtherActor :type "Actor Object Reference") (OtherComponent :type "SceneComponent Object Reference"))
  (returns (IsShoot :type Boolean))
  (if (`KismetStringLibrary.Contains` (`KismetSystemLibrary.GetDisplayName` OtherComponent) "ArrowBox")
    (bind _asbp_arrow (cast `/Game/VR_Archery/Blueprint/BowAndArrow/BP_Arrow` OtherActor))
    (`PrimitiveComponent.SetCollisionEnabled` (`/Game/VR_Archery/Blueprint/BowAndArrow/BP_Arrow.ArrowBox` _asbp_arrow) "NoCollision")
    (return true)
    (else
      (return false))))

(fn `UserConstructionScript`)