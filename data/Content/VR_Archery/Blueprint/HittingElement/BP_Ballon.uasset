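; Balloon target for VR archery that floats upward until it is shot or climbs out of range.
; Tick raises the mesh at a constant speed and destroys the actor past a height limit.
; An overlap with an arrow's box, matched by component name substring, hides and disables collision on both arrow and balloon.
; The hit also plays a sound, then destroys the balloon after a delay.
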(event `self.StaticMeshComponent.OnComponentBeginOverlap`
  (params (OverlappedComponent :type "PrimitiveComponent Object Reference") (OtherActor :type "Actor Object Reference") (OtherComp :type "PrimitiveComponent Object Reference") (OtherBodyIndex :type Integer) (bFromSweep :type Boolean) (SweepResult :type "HitResult Structure (by ref)"))
  (if (`KismetStringLibrary.Contains` (`KismetSystemLibrary.GetDisplayName` OtherComp) "ArrowBox")
    (bind _asbp_arrow (cast `/Game/VR_Archery/Blueprint/BowAndArrow/BP_Arrow` OtherActor))
    (`SceneComponent.SetVisibility` (`Actor.RootComponent` _asbp_arrow) false false)
    (`PrimitiveComponent.SetCollisionEnabled` (`/Game/VR_Archery/Blueprint/BowAndArrow/BP_Arrow.ArrowBox` _asbp_arrow) "NoCollision")
    (`SceneComponent.SetVisibility` (`self.StaticMeshComponent`) false true)
    (`PrimitiveComponent.SetCollisionEnabled` (`self.StaticMeshComponent`) "NoCollision")
    (`AudioComponent.Play` (`self.Audio`) 0.0)
    (`KismetSystemLibrary.Delay` 5.0)
    (`self.K2_DestroyActor`)))

(event `self.ReceiveTick`
  (params (DeltaSeconds :type "Float (single-precision)"))
  (bind (_returnvalue_x _returnvalue_y _returnvalue_z) (`KismetMathLibrary.BreakVector` (`SceneComponent.K2_GetComponentLocation` (`self.StaticMeshComponent`))))
  (`SceneComponent.K2_SetWorldLocation` (`self.StaticMeshComponent`) (`KismetMathLibrary.MakeVector` _returnvalue_x _returnvalue_y (+ _returnvalue_z (* DeltaSeconds 20.0))) false false)
  (if (> _returnvalue_z 2000.0)
    (`self.K2_DestroyActor`)))

(fn `UserConstructionScript`)