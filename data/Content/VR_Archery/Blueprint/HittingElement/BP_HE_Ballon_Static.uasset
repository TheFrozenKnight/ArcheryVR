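; Static balloon target for the VR archery game that pops when hit by an arrow and respawns after a delay.
; An overlap from an arrow's ArrowBox component hides the arrow and balloon with string, disables their collision and plays the pop audio.
; Five seconds later the balloon reappears with collision restored and a random color material, which is also picked on BeginPlay.
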(event `self.ReceiveBeginPlay`
  (`self.RefreshMaterial`))

(event `self.SM_Balloon.OnComponentBeginOverlap`
  (params (OverlappedComponent :type "PrimitiveComponent Object Reference") (OtherActor :type "Actor Object Reference") (OtherComp :type "PrimitiveComponent Object Reference") (OtherBodyIndex :type Integer) (bFromSweep :type Boolean) (SweepResult :type "HitResult Structure (by ref)"))
  (bind _output_get (set `self.Other Actor` OtherActor))
  (if (`KismetStringLibrary.Contains` (`KismetSystemLibrary.GetDisplayName` OtherComp) "ArrowBox")
    (bind _asbp_arrow (cast `/Game/VR_Archery/Blueprint/BowAndArrow/BP_Arrow` _output_get))
    (`SceneComponent.SetVisibility` (`Actor.RootComponent` _asbp_arrow) false false)
    (`PrimitiveComponent.SetCollisionEnabled` (`/Game/VR_Archery/Blueprint/BowAndArrow/BP_Arrow.ArrowBox` _asbp_arrow) "NoCollision")
    (`SceneComponent.SetVisibility` (`self.SM_String`) false true)
    (`SceneComponent.SetVisibility` (`self.SM_Balloon`) false true)
    (`PrimitiveComponent.SetCollisionEnabled` (`self.SM_Balloon`) "NoCollision")
    (`AudioComponent.Play` (`self.Audio`) 0.0)
    (`KismetSystemLibrary.Delay` 5.0)
    (`SceneComponent.SetVisibility` (`self.SM_String`) true true)
    (`SceneComponent.SetVisibility` (`self.SM_Balloon`) true true)
    (`PrimitiveComponent.SetCollisionEnabled` (`self.SM_Balloon`) "QueryOnly")
    (`self.RefreshMaterial`)))

(fn `RefreshMaterial`
  (`PrimitiveComponent.SetMaterial` (`self.SM_Balloon`) 0 (`|GetArrayItem` (`self.Color`) (`KismetMathLibrary.RandomInteger` 6))))

(fn `UserConstructionScript`)